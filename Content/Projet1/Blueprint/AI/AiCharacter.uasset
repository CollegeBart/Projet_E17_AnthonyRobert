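; AiCharacter is an AI character Blueprint with a configurable body mesh, hit points and hit flash feedback.
; Construction applies VariableMesh and a dynamic instance of MeshMat, or prints a warning when no mesh is set.
; Any damage reduces HitPoints and destroys the actor at zero or below.
; Every Hit event briefly swaps in HitFlash, then restores plain MeshMat; an ApplyDamage call to the hit actor is unreachable.
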(event `self.ReceiveAnyDamage`
  (params (Damage :type "Float (single-precision)") (DamageType :type "DamageType Object Reference") (InstigatedBy :type "Controller Object Reference") (DamageCauser :type "Actor Object Reference"))
  ;[1 1 1] Do Damage
  (set `self.HitPoints` (- (`self.HitPoints`) Damage))
  (if (<= (`self.HitPoints`) 0.0)
    (`self.K2_DestroyActor`)))

(event `self.ReceiveHit`
  (params (MyComp :type "PrimitiveComponent Object Reference") (Other :type "Actor Object Reference") (OtherComp :type "PrimitiveComponent Object Reference") (bSelfMoved :type Boolean) (HitLocation :type "Vector Structure") (HitNormal :type "Vector Structure") (NormalImpulse :type "Vector Structure") (Hit :type "HitResult Structure (by ref)"))
  ;[1 1 1] Get Hit Flash for feedback
  (if true
    (`PrimitiveComponent.SetMaterial` (`self.body`) 0 "/Game/Projet1/Blueprint/Material/HitFlash.HitFlash")
    (`KismetSystemLibrary.Delay` 0.08)
    (`PrimitiveComponent.SetMaterial` (`self.body`) 0 (`self.MeshMat`))))

(fn `UserConstructionScript`
  (bind _variablemesh (`self.VariableMesh`))
  (if (== _variablemesh null)
    (`KismetSystemLibrary.PrintString` "Please set variable mesh before usage")
    (else
      (`StaticMeshComponent.SetStaticMesh` (`self.body`) _variablemesh)
      (bind _returnvalue (`KismetMaterialLibrary.CreateDynamicMaterialInstance` (`self.MeshMat`)))
      (`PrimitiveComponent.SetMaterial` (`self.body`) 0 _returnvalue))))