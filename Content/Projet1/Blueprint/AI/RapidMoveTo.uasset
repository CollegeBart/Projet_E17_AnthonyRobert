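; Behavior Tree task that moves a FollowerIcon-controlled pawn toward the actor stored in the TargetToFollow blackboard key.
; On execute, it casts the owner to FollowerIcon, caches it and starts AI MoveTo, but only while that cached reference is unset.
; A successful move finishes the task as failed; move failure, a failed cast and an already-set reference never finish it.
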(event `self.ReceiveExecute`
  (params (OwnerActor :type "Actor Object Reference"))
  (if (not (!= (`self.AI_CON_Ref`) null))
    (bind _asfollower_icon (cast `/Game/Projet1/Blueprint/AI/FollowerIcon` OwnerActor))
    (set `self.AI_CON_Ref` _asfollower_icon)
    (`|AIMoveTo` (`Controller.K2_GetPawn` (`self.AI_CON_Ref`)) (0.0 0.0 0.0) (`BTFunctionLibrary.GetBlackboardValueAsActor` (`self.TargetToFollow`))
      (:`OnSuccess`
        (`self.FinishExecute` false)))))