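; BasicEnemy is an enemy Blueprint with configurable mesh and hit points that awards score through TopDownMode when killed.
; Incoming damage briefly flashes the body with HitFlash before restoring MeshMat, or destroys the actor at zero health.
; Any capsule overlap damages the player pawn, without checking which actor overlapped.
; The construction script applies VariableMesh and a dynamic material instance, printing a warning if the mesh is unset.
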(event `self.ReceiveAnyDamage`
  (params (Damage :type "Float (single-precision)") (DamageType :type "DamageType Object Reference") (InstigatedBy :type "Controller Object Reference") (DamageCauser :type "Actor Object Reference"))
  ;[1 1 1] Do damage
  (bind _output_get (set `self.HitPoints` (- (`self.HitPoints`) Damage)))
  (if (<= _output_get 0.0)
    (bind _astop_down_mode (cast `/Game/Projet1/Blueprint/TopDownMode` (`GameplayStatics.GetGameMode`)))
    (`/Game/Projet1/Blueprint/TopDownMode.IncrementScore` _astop_down_mode 200)
    (`self.K2_DestroyActor`)
    (else
      (`PrimitiveComponent.SetMaterial` (`self.Body`) 0 "/Game/Projet1/Blueprint/Material/HitFlash.HitFlash")
      (`KismetSystemLibrary.Delay` 0.08)
      (`PrimitiveComponent.SetMaterial` (`self.Body`) 0 (`self.MeshMat`)))))

(event `self.CapsuleComponent.OnComponentBeginOverlap`
  (params (OverlappedComponent :type "PrimitiveComponent Object Reference") (OtherActor :type "Actor Object Reference") (OtherComp :type "PrimitiveComponent Object Reference") (OtherBodyIndex :type Integer) (bFromSweep :type Boolean) (SweepResult :type "HitResult Structure (by ref)"))
  (`GameplayStatics.ApplyDamage` (`GameplayStatics.GetPlayerPawn` 0) (`self.Damage`) null OtherActor))

(fn `UserConstructionScript`
  (bind _variablemesh (`self.VariableMesh`))
  (if (== _variablemesh null)
    (`KismetSystemLibrary.PrintString` "Please set variable mesh before usage")
    (else
      (`StaticMeshComponent.SetStaticMesh` (`self.Body`) _variablemesh)
      (bind _returnvalue (`KismetMaterialLibrary.CreateDynamicMaterialInstance` (`self.MeshMat`)))
      (`PrimitiveComponent.SetMaterial` (`self.Body`) 0 _returnvalue))))