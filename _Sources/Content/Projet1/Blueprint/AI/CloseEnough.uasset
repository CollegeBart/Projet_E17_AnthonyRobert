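; CloseEnough is a behavior tree decorator that gates follower AI logic on the distance to its follow target.
; It casts the owner to FollowerIcon, then measures the distance from its controlled pawn to the TargetToFollow blackboard actor.
; Despite the name, the condition passes when that distance is at least AcceptableDistance, meaning the follower is not yet close enough.
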(fn `PerformConditionCheck`
  (params (OwnerActor :type "Actor Object Reference"))
  (returns (ReturnValue :type Boolean))
  (bind _asfollower_icon (cast `/Game/Projet1/Blueprint/AI/FollowerIcon` OwnerActor))
  (set `self.AI_CON_Ref` _asfollower_icon)
  (return (>= (`KismetMathLibrary.VSize` (- (`Actor.K2_GetActorLocation` (`BTFunctionLibrary.GetBlackboardValueAsActor` (`self.TargetToFollow`))) (`Actor.K2_GetActorLocation` (`Controller.K2_GetPawn` (`self.AI_CON_Ref`))))) (`self.AcceptableDistance`))))