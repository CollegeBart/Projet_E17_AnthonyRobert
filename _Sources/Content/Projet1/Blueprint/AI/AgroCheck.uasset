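; AI aggro-check Blueprint, apparently a behavior tree service, for the FollowerIcon controller.
; On tick it caches the controller, gathers actors and stores the pawn's location, then stops.
; An unconnected chain would sphere-trace for objects, line-trace each hit for visibility and write TargetToFollow and TargetLocation to the blackboard.
; That detection never runs, and its TargetToFollow writes pass no object.
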(event `self.ReceiveTick`
  (params (OwnerActor :type "Actor Object Reference") (DeltaSeconds :type "Float (single-precision)"))
  ;[1 1 1] Is AI_CON_Ref set ?
  (if (not (!= (`self.AI_CON_Ref`) null))
    (bind _asfollower_icon (cast `/Game/Projet1/Blueprint/AI/FollowerIcon` OwnerActor))
    (set `self.AI_CON_Ref` _asfollower_icon))
  (bind _outactors (`GameplayStatics.GetAllActorsOfClass` null))
  (set `self.MyLocation` (`Actor.K2_GetActorLocation` (`Controller.K2_GetPawn` (`self.AI_CON_Ref`)))))